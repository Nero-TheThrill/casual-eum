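; Ice cube spawner that creates BP_IceCube actors from a queue of requested spawn transforms, one at a time with a cooldown.
; QueueOneIceCube adds transforms, and Tick arms a one-shot timer whenever the queue has entries and no timer is pending.
; SpawnIceCube spawns and attaches the front entry, dequeues it and clears the timer handle.
; TestFunc, run at BeginPlay and after each spawn, stomps the first attached cube.
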(event EventBeginPlay
  (CallFunction|TestFunc))

(event Collision|EventActorBeginOverlap
  (params (OtherActor :type Actor%20Object%20Reference)))

(event EventTick
  (params (DeltaSeconds :type Float%20%28single-precision%29))
  (if (not (CallFunction|IsQueueEmpty))
    (if (not (Utilities|Time|IsValidTimerHandle (Variables|Default|GetSpawnTimerHandle)))
      (bind _returnvalue (Utilities|Time|SetTimerbyFunctionName 0 "SpawnIceCube" (Variables|Default|GetSpawnCoolTime)))
      (Variables|Default|SetSpawnTimerHandle _returnvalue)
      (Variables|Default|SetElapsedTime 0.0))))

(fn ConstructionScript)

(fn QueueOneIceCube
  (params (SpawnTransform :type Transform))
  (Utilities|Array|Add (Variables|Default|GetSpawnTransformQueue) SpawnTransform))

(fn IsQueueEmpty
  (return (== (Utilities|Array|Length (Variables|Default|GetSpawnTransformQueue)) 0)))

(fn SpawnIceCube
  (bind _returnvalue (Game|SpawnActorfromClass "/Game/Game/BP_IceCube.BP_IceCube_C" (Utilities|Array|Get(acopy) (Variables|Default|GetSpawnTransformQueue)) "AdjustIfPossibleButAlwaysSpawn" "OverrideRootScale" 0 0))
  (Transformation|AttachActorToActor _returnvalue self "None" "KeepWorld" "KeepWorld" "KeepWorld" true)
  (Utilities|Array|RemoveIndex (Variables|Default|GetSpawnTransformQueue))
  (Utilities|Time|InvalidateTimerHandle (Variables|Default|GetSpawnTimerHandle))
  (CallFunction|TestFunc))

(fn TestFunc
  (bind _asbp_ice_cube (Utilities|Casting|CastToBP_IceCube (Utilities|Array|Get(acopy) (Actor|GetAttachedActors true false))))
  (Default|OnStomped _asbp_ice_cube))