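; BP_IceCube1 is an ice cube actor that can be stomped loose and then caught in a hand.
; OnStomped tells the parent BP_IceCubeSpawner to queue a cube at this transform, then enables mesh physics; without that parent, nothing happens.
; OnCatched detaches the cube, attaches it to the given component's right-hand socket, stops physics and destroys it after a short timer.
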(event EventBeginPlay)

(event Collision|EventActorBeginOverlap
  (params (OtherActor :type Actor%20Object%20Reference)))

(event EventTick
  (params (DeltaSeconds :type Float%20%28single-precision%29)))

(fn ConstructionScript)

(fn OnStomped
  (bind _asbp_ice_cube_spawner (Utilities|Casting|CastToBP_IceCubeSpawner (Actor|GetAttachParentActor)))
  (Default|QueueOneIceCube _asbp_ice_cube_spawner (Transformation|GetActorTransform))
  (Development|PrintString "213")
  (Physics|SetSimulatePhysics (Variables|Default|Geticecube_fbx) true))

(fn OnCatched
  (params (AttachComp :type Mesh%20Component%20Object%20Reference))
  (Transformation|DetachFromActor "KeepWorld" "KeepWorld" "KeepWorld")
  (Transformation|AttachComponentToComponent AttachComp "hand_rSocket" "KeepWorld" "KeepWorld" "KeepWorld" false)
  (Physics|SetSimulatePhysics (Variables|Default|Geticecube_fbx) false)
  (Utilities|Time|SetTimerbyFunctionName 0 "Dead" 1.0))

(fn Dead
  (Actor|DestroyActor))