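; BP_DefenderController is a player controller that turns Enhanced Input actions into movement and catching for the defender character.
; On BeginPlay it adds the IMC_Defender mapping context.
; IA_MoveRight prints its value and moves the controlled pawn along the controller's own forward vector, despite the action's name.
; IA_Catch casts the pawn to BP_DefenderCharacter and calls StartCatching, leaving the catch logic to the character.
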(event Input|EnhancedActionEvents|EnhancedInputActionIA_MoveRight
  (params (ActionValue :type Float%20%28double-precision%29) (ElapsedSeconds :type Float%20%28double-precision%29) (TriggeredSeconds :type Float%20%28double-precision%29) (InputAction :type Input%20Action%20Object%20Reference :default "/Game/Input/IA_MoveRight.IA_MoveRight"))
  (Development|PrintString (Utilities|String|ToString(Float) ActionValue))
  (Pawn|Input|AddMovementInput (Pawn|GetControlledPawn) (Transformation|GetActorForwardVector) ActionValue false))

(event Input|EnhancedActionEvents|EnhancedInputActionIA_Catch
  (params (ActionValue :type Boolean) (ElapsedSeconds :type Float%20%28double-precision%29) (TriggeredSeconds :type Float%20%28double-precision%29) (InputAction :type Input%20Action%20Object%20Reference :default "/Game/Input/IA_Catch.IA_Catch"))
  (bind _asbp_defender_character (Utilities|Casting|CastToBP_DefenderCharacter (Pawn|GetControlledPawn)))
  (Default|StartCatching _asbp_defender_character))

(event EventBeginPlay
  (Input|AddMappingContext (PlayerController|LocalPlayerSubsystems|GetEnhancedInputLocalPlayerSubsystem) "/Game/Input/IMC_Defender.IMC_Defender" 0 "(bIgnoreAllPressedKeysUntilRelease=True,bForceImmediately=False,bNotifyUserSettings=False)"))

(event EventTick
  (params (DeltaSeconds :type Float%20%28single-precision%29)))

(fn ConstructionScript)