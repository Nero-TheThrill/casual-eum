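; Character Blueprint that provides helper functions for forward/backward movement and direction checking.
; BeginPlay caches the actor's initial forward vector as WorldForward.
; IsForwardDirection uses a dot product to test whether the current forward, multiplied by an input scale, points along that cached vector.
; MoveForwardBackward adds movement input along the current forward at full scale, ignoring its Scale parameter; neither function is called within this graph.
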(event EventBeginPlay
  (Variables|Default|SetWorldForward (Transformation|GetActorForwardVector)))

(event Collision|EventActorBeginOverlap
  (params (OtherActor :type Actor%20Object%20Reference)))

(fn ConstructionScript)

(fn MoveForwardBackward
  (params (Scale :type Float%20%28double-precision%29))
  (Pawn|Input|AddMovementInput (Transformation|GetActorForwardVector) 1.0 false))

(fn IsForwardDirection
  (params (InputScale :type Float%20%28double-precision%29))
  (return (> (Math|Vector|DotProduct (Variables|Default|GetWorldForward) (* (Transformation|GetActorForwardVector) InputScale)) 0.0)))