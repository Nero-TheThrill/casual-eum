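; BP_AttackerController is the controller for the attacker, handling movement input for a BP_Character pawn.
; On BeginPlay it adds the IMC_Attacker Enhanced Input mapping context and caches the controlled pawn as BP_Character.
; IA_Move asks the character whether the input points forward: if so it calls MoveForwardBackward, otherwise it flips the control rotation yaw by 180 degrees to turn around.
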(event Input|EnhancedActionEvents|EnhancedInputActionIA_Move
  (params (ActionValue :type Float%20%28double-precision%29) (ElapsedSeconds :type Float%20%28double-precision%29) (TriggeredSeconds :type Float%20%28double-precision%29) (InputAction :type Input%20Action%20Object%20Reference :default "/Game/Input/IA_Move.IA_Move"))
  (bind _returnvalue (Pawn|GetControlRotation :!class /Script/Engine.Controller))
  (if (Default|IsForwardDirection (Variables|Default|GetControlledPawn) ActionValue)
    (Default|MoveForwardBackward (Variables|Default|GetControlledPawn) ActionValue)
    (else
      (Pawn|SetControlRotation (Math|Rotator|MakeRotator (.roll _returnvalue) (.pitch _returnvalue) (+ (.yaw _returnvalue) 1.8e+02))))))

(event EventBeginPlay
  (Input|AddMappingContext (PlayerController|LocalPlayerSubsystems|GetEnhancedInputLocalPlayerSubsystem) "/Game/Input/IMC_Attacker.IMC_Attacker" 0 "(bIgnoreAllPressedKeysUntilRelease=True,bForceImmediately=False,bNotifyUserSettings=False)")
  (bind _asbp_character (Utilities|Casting|CastToBP_Character (Pawn|GetControlledPawn)))
  (Variables|Default|SetControlledPawn _asbp_character))

(event EventTick
  (params (DeltaSeconds :type Float%20%28single-precision%29)))

(fn ConstructionScript)